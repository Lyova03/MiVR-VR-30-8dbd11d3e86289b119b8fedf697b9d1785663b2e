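; BP_CustomProduct is an actor representing a customizable product assembled from named part actors in its Parts array.
; CreatePart spawns a BP_CustomProductPart with static mesh components and materials, calling AddPart inside the mesh loop to store and attach it.
; Name lookups drive part removal, with optional destruction, and per-part material swaps on slot 0.
; SetColor temporarily ignores the part name, writing a shared material parameter collection instead.
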(event `self.ReceiveBeginPlay`)

(fn `AddPart`
  (params (part :type "/Game/VRBase/Blueprints/BP_CustomProductPart Object Reference"))
  (returns (Index :type Integer))
  (bind _returnvalue (`KismetArrayLibrary.Array_Add` (`self.Parts`) part))
  (`self.K2_AttachToActor` part self "None" "KeepRelative" "KeepRelative" "KeepRelative" true)
  (return _returnvalue))

(fn `CreatePart`
  (params (Name :type Name) (Meshes :type "Array of StaticMesh Object Reference") (Materials :type "Array of MaterialInstance Object Reference"))
  (returns (Part :type "/Game/VRBase/Blueprints/BP_CustomProductPart Object Reference"))
  (bind _returnvalue (`|SpawnActorFromClass` "/Game/VRBase/Blueprints/BP_CustomProductPart.BP_CustomProductPart_C" (`KismetMathLibrary.MakeTransform` (0.0 0.0 0.0)) "Undefined" "OverrideRootScale"))
  (set `/Game/VRBase/Blueprints/BP_CustomProductPart.Name` Name _returnvalue)
  (for (_array_element _array_index) Meshes
    (bind _returnvalue_2 (`AddComponent|StaticMeshComponent_1` :`self` _returnvalue))
    (`StaticMeshComponent.SetStaticMesh` _returnvalue_2 _array_element)
    (`PrimitiveComponent.SetMaterial` _returnvalue_2 0 (`KismetArrayLibrary.Array_Get` Materials _array_index))
    (`self.AddPart` _returnvalue))
  (return _returnvalue))

(fn `Find`
  (params (Name :type Name))
  (returns (Part :type "/Game/VRBase/Blueprints/BP_CustomProductPart Object Reference"))
  (for _array_element (`self.Parts`)
    (if (== (`/Game/VRBase/Blueprints/BP_CustomProductPart.Name` _array_element) Name)
      (return _array_element)))
  (return null))

(fn `FindIndex`
  (params (Name :type Name))
  (returns (Index :type Integer))
  (for (_array_element _array_index) (`self.Parts`)
    (if (== (`/Game/VRBase/Blueprints/BP_CustomProductPart.Name` _array_element) Name)
      (return _array_index)))
  (return -1))

(fn `GetNumberParts`
  (returns (Length :type Integer))
  (return (`KismetArrayLibrary.Array_Length` (`self.Parts`))))

(fn `RemovePart`
  (params (Name :type Name) (Destroy :type Boolean :default false))
  (locals (ProductToRemove :type "/Game/VRBase/Blueprints/BP_CustomProductPart Object Reference"))
  (`|ExecutionSequence`
    (:`then_0`
      (bind _index (`self.FindIndex` Name))
      (if (not (>= _index 0))
        (return)))
    (:`then_1`
      (bind _output_get (set `local.ProductToRemove` (`KismetArrayLibrary.Array_Get` (`self.Parts`) _index))))
    (:`then_2`
      (`self.K2_DetachFromActor` _output_get "KeepRelative" "KeepRelative" "KeepRelative"))
    (:`then_3`
      (if Destroy
        (`self.K2_DestroyActor` _output_get)))
    (:`then_4`
      (`KismetArrayLibrary.Array_Remove` (`self.Parts`) _index)
      (return))))

(fn `SetColor`
  (params (PartName :type Name) (Color :type "Vector Structure"))
  ;[1 1 1] Temporary solution
  (`KismetMaterialLibrary.SetVectorParameterValue` "/Game/cgMaterials/Base/BaseMaterialCollection.BaseMaterialCollection" "BaseColorVector" (`KismetMathLibrary.Conv_VectorToLinearColor` Color)))

(fn `SetMaterial`
  (params (PartName :type Name) (Material :type "MaterialInstance Object Reference"))
  (`|ExecutionSequence`
    (:`then_0`
      (bind _index (`self.FindIndex` PartName))
      (if (< _index 0)
        (return)))
    (:`then_1`
      (for _array_element (`self.K2_GetComponentsByClass` (`KismetArrayLibrary.Array_Get` (`self.Parts`) _index) "/Script/Engine.StaticMeshComponent")
        (`PrimitiveComponent.SetMaterial` _array_element 0 Material))
      (return))))

(fn `UserConstructionScript`)