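; Actor component that makes its owning actor grabbable in VR, with Pickup called by BP_MotionController.
; Pickup attaches the owner's root to the given component, keeping world transform, and disables static and skeletal mesh physics if that attach target is simulating.
; Drop detaches the owner and restores physics if Pickup disabled it.
; Pickup also prints a repeated "Hello" debug message.
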(event `SetSimulatePhysics`
  (params (bSimulate :type Boolean))
  (bind _returnvalue (`self.GetOwner`))
  (`PrimitiveComponent.SetSimulatePhysics` (`Actor.K2_GetComponentsByClass` _returnvalue "/Script/Engine.StaticMeshComponent") bSimulate)
  (`PrimitiveComponent.SetSimulatePhysics` (`Actor.K2_GetComponentsByClass` _returnvalue "/Script/Engine.SkeletalMeshComponent") bSimulate))

(event `/Game/VRBase/Blueprints/PickupActorInterface.Pickup`
  (params (AttachTo :type "SceneComponent Object Reference"))
  (for _ (range 11)
    (`KismetSystemLibrary.PrintString` "Hello"))
  (bind _output_get (set `self.IsSimulated?` (`self.IsSimulatingPhysics` AttachTo "None")))
  (if _output_get
    (`self.SetSimulatePhysics` false))
  (`self.K2_AttachToComponent` (`Actor.K2_GetRootComponent` (`self.GetOwner`)) AttachTo "None" "KeepWorld" "KeepWorld" "KeepWorld" false))

(event `/Game/VRBase/Blueprints/PickupActorInterface.Drop`
  (if (`self.IsSimulated?`)
    (`self.SetSimulatePhysics` true)
    (set `self.IsSimulated?` false))
  (`Actor.K2_DetachFromActor` (`self.GetOwner`) "KeepWorld" "KeepWorld" "KeepWorld"))